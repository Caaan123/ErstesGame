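; BP_TestTarget is a test dummy enemy that wanders and can be damaged and killed repeatedly.
; DummyHit subtracts Damage from Health and prints the remainder, or calls Death when health would reach zero.
; Death briefly hides the character mesh, then restores health and visibility without destroying the actor.
; From BeginPlay, AIMove moves to random nearby reachable points, re-triggering itself only when a move succeeds.
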(event Custom|Death
  (Rendering|SetVisibility (Variables|Default|GetCharacterMesh) false true)
  (Utilities|FlowControl|Delay 0.1)
  (Variables|Default|SetHealth 1e+02)
  (Rendering|SetVisibility (Variables|Default|GetCharacterMesh) true true))

(event Custom|DummyHit
  (Utilities|FlowControl|Sequence
    (:then_0
      (bind _output_get (Variables|Default|SetNewHealth (- (Variables|Default|GetHealth) (Variables|Default|GetDamage))))
      (if (<= _output_get 0.0)
        (CallFunction|Death)
        (else
          (bind _output_get_2 (Variables|Default|SetHealth _output_get))
          (Development|PrintString (Utilities|String|ToString(Float) _output_get_2)))))))

(event Custom|AIMove
  (AI|AIMoveTo self (.RandomLocation (AI|Navigation|GetRandomReachablePointinRadius (Transformation|GetActorLocation) 2.5e+02 0 0)) 0 5.0 true
    (:OnSuccess
      (CallFunction|AIMove))))

(event Collision|EventActorBeginOverlap
  (params (OtherActor :type Actor%20Object%20Reference)))

(event EventBeginPlay
  (CallFunction|AIMove))

(fn ConstructionScript)